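; BP_Player is the player of a shooter, moving along its right and up axes from input and firing bullets.
; Tick applies normalized, frame-rate independent movement without sweep.
; Holding Fire shoots immediately and repeats on a looping timer, each shot spawning BP_Bullet at the Arrow with a sound.
; SetHP updates the HP widget at BeginPlay and on DoDamage, which reports whether HP is depleted.
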(event `self.ReceiveBeginPlay`
  ;[1 1 1] 태어날 때 체력을 최대 체력으로 하고싶다.
  (`self.SetHP` (`self.MaxHp`)))

(event `self.ReceiveTick`
  (params (DeltaSeconds :type "Float (single-precision)"))
  (`|ExecutionSequence`
    (:`then_0`
      ;[1 1 1] 사용자의 입력에따라 이동하고싶다.P = P0 + vt (다음위치 = 현재위치 + 속도(방향*크기) * 시간)
      (`self.Translate` (`self.GetDirection`) (`self.Speed`)))))

(event `InputAction|Fire`
  (params (Key :type "Key Structure"))
  (:`Pressed`
    (bind _returnvalue (`KismetSystemLibrary.K2_SetTimer` null "MakeBullet" (`self.FireInterval`) true))
    (set `self.MakeBulletTimerHandle` _returnvalue)
    (`self.MakeBullet`))
  (:`Released`
    (`KismetSystemLibrary.K2_ClearAndInvalidateTimerHandle` (`self.MakeBulletTimerHandle`))))

(fn `DoDamage`
  (params (damage :type Integer))
  (returns (IsDie :type Boolean))
  (`self.SetHP` (- (`self.HP`) damage))
  (return (<= (`self.HP`) 0)))

(fn `GetDirection`
  (returns (Direction :type "Vector Structure"))
  (return (`KismetMathLibrary.Normal` (+ (* (`self.GetInputAxisValue`) (`self.GetActorRightVector`)) (* (`self.GetInputAxisValue`) (`self.GetActorUpVector`))))))

(fn `MakeBullet`
  (`|SpawnActorFromClass` "/Game/Blueprints/BP_Bullet.BP_Bullet_C" (`SceneComponent.K2_GetComponentToWorld` (`self.Arrow`)) "AlwaysSpawn" "MultiplyWithRoot" null null)
  (`GameplayStatics.PlaySound2D` "/Game/Sounds/star-wars-blaster.star-wars-blaster" 1.0 1.0 0.0 null null))

(fn `SetHP`
  (params (Value :type Integer))
  (set `self.HP` Value)
  (bind _aswbp_player_hp (cast `/Game/Blueprints/WBP_PlayerHP` (`WidgetComponent.GetWidget` (`self.WidgetHP`))))
  (`/Game/Blueprints/WBP_PlayerHP.Update HP` _aswbp_player_hp (`KismetMathLibrary.Conv_IntToDouble` (`self.HP`)) (`KismetMathLibrary.Conv_IntToDouble` (`self.MaxHp`))))

(fn `Translate`
  (params (Direction :type "Vector Structure") (Speed :type "Float (double-precision)") (IsSweep :type Boolean))
  (`self.K2_SetActorLocation` (+ (`self.K2_GetActorLocation`) (* Speed (`KismetMathLibrary.Normal` Direction) (`GameplayStatics.GetWorldDeltaSeconds`))) IsSweep))

(fn `UserConstructionScript`)