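; BP_Enemy is an enemy actor that flies in a straight line and explodes when it overlaps the player.
; On spawn it picks a fixed direction, aimed at the player 30% of the time and forward otherwise, then moves via a frame-rate-independent Translate helper.
; Overlapping BP_Player triggers effects, damage and self-destruction.
; If DoDamage returns true, it also destroys the player and, after a delay, pauses the game and shows the game-over widget.
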(event `self.ReceiveBeginPlay`
  ;[1 1 1] 태어날 때 방향을 정하고 싶다.
  ;  30% 확률로 플레이어를 향하는 방향
  ;  나머지 확률로 앞 방향
  (if (< (`KismetMathLibrary.RandomIntegerInRange` 0 9) 3)
    (set `self.Direction` (`KismetMathLibrary.Normal` (- (`self.K2_GetActorLocation` (`GameplayStatics.GetPlayerPawn` 0)) (`self.K2_GetActorLocation`))))
    (else
      (set `self.Direction` (`self.GetActorForwardVector`)))))

(event `self.ReceiveTick`
  (params (DeltaSeconds :type "Float (single-precision)"))
  ;[1 1 1] 살아가면서 정한 방향으로 계속 이동하고싶다.
  (`self.Translate` (`self.Direction`) (`self.Speed`))
  (`self.K2_SetActorRotation` (`KismetMathLibrary.MakeRotFromXZ` (`self.Direction`) (`self.GetActorUpVector`))))

(event `self.ReceiveActorBeginOverlap`
  (params (OtherActor :type "Actor Object Reference"))
  (bind _returnvalue (`GameplayStatics.GetPlayerController` 0))
  (bind _asbp_player (cast `/Game/Blueprints/BP_Player` OtherActor))
  ;[1 1 1] 부딪힌 상대가 플레이어라면 부딪힌 위치에 폭발 VFX를 표현하고 너죽고 나죽고 하고싶다. 게임을 일시정지 시키고싶다.
  (`GameplayStatics.SpawnEmitterAtLocation` "/Game/StarterContent/Particles/P_Explosion.P_Explosion" (`self.K2_GetActorLocation`))
  (`GameplayStatics.PlaySound2D` "/Game/Sounds/Explosion.Explosion" 1.0 1.0 0.0 null null)
  (bind _isdie (`/Game/Blueprints/BP_Player.DoDamage` _asbp_player 10))
  (if _isdie
    (`self.K2_DestroyActor` _asbp_player)
    (`KismetSystemLibrary.Delay` 1.0)
    (`self.K2_DestroyActor`)
    (`GameplayStatics.SetGamePaused` true)
    (bind _returnvalue_2 (`|CreateWidget` "/Game/Blueprints/WBP_GameOver.WBP_GameOver_C"))
    (`UserWidget.AddToViewport` _returnvalue_2 0)
    (set `PlayerController.bShowMouseCursor` true _returnvalue)
    (`WidgetBlueprintLibrary.SetInputMode_UIOnlyEx` _returnvalue null)
    (else
      (`self.K2_DestroyActor`))))

(fn `Translate`
  (params (Direction :type "Vector Structure") (Speed :type "Float (double-precision)") (IsSweep :type Boolean))
  (`self.K2_SetActorLocation` (+ (`self.K2_GetActorLocation`) (* Speed (`KismetMathLibrary.Normal` Direction) (`GameplayStatics.GetWorldDeltaSeconds`))) IsSweep))

(fn `UserConstructionScript`)