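; BP_EnemyManager is a spawner actor that creates enemies at a fixed interval while the player is alive.
; On BeginPlay it starts a looping timer that calls MakeEnemy every MakeTime seconds and stores the handle.
; MakeEnemy spawns BP_Enemy at the Arrow component's transform, or clears the timer once the player pawn is no longer valid.
; A Tick-based accumulator and an event-bound timer remain as disconnected, unused alternatives.
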(event `self.ReceiveBeginPlay`
  (bind _returnvalue (`KismetSystemLibrary.K2_SetTimer` null "MakeEnemy" (`self.MakeTime`) true))
  (set `self.TimerHandMakeEnemy` _returnvalue))

(event `CustomEvent MakeEnemy`
  (`self.MakeEnemy`))

(event `self.ReceiveTick`
  (params (DeltaSeconds :type "Float (single-precision)"))
  ;[1 1 1] 시간이 흐르다가 현재시간이 생성시간이 되면 적을 Arrow위치에 스폰하고싶다. 현재시간을 0으로 초기화 하고싶다.
)

(fn `MakeEnemy`
  ;[1 1 1] 플레이어가 죽었다면 더 이상 적을 만들지 않고 싶다.
  (`/Engine/EditorBlueprintResources/StandardMacros.IsValid` (`GameplayStatics.GetPlayerPawn` 0)
    (:`Is Valid`
      (`|SpawnActorFromClass` "/Game/Blueprints/BP_Enemy.BP_Enemy_C" (`SceneComponent.K2_GetComponentToWorld` (`self.Arrow`)) "AlwaysSpawn" "MultiplyWithRoot" null null))
    (:`Is Not Valid`
      (`KismetSystemLibrary.K2_ClearAndInvalidateTimerHandle` (`self.TimerHandMakeEnemy`)))))

(fn `UserConstructionScript`)