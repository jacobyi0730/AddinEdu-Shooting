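; BP_ShootingGameModeBase is the shooting game's mode, tracking the score and high score.
; On BeginPlay it shows the WBP_Score widget, hides the mouse cursor and sets game-only input.
; AddScore accumulates points and raises HighScore whenever Score exceeds it.
; SaveHighScore writes HighScore into a new BP_SaveGame and saves it to a slot, while LoadHighScore is still an empty stub.
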(event `self.ReceiveBeginPlay`
  (bind _returnvalue (`GameplayStatics.GetPlayerController` 0))
  ;[1 1 1] WBP_Score를 화면에 보이게하고싶다.
  (bind _returnvalue_2 (`|CreateWidget` "/Game/Blueprints/WBP_Score.WBP_Score_C"))
  (`UserWidget.AddToViewport` _returnvalue_2 0)
  ;[1 1 1] 마우스커서를 숨기고싶다. 입력을 게임창에서 받고싶다.
  (set `PlayerController.bShowMouseCursor` false _returnvalue)
  (`WidgetBlueprintLibrary.SetInputMode_GameOnly` _returnvalue))

(fn `AddScore`
  (params (Value :type Integer))
  ;[1 1 1] Score에 Value를 누적하고싶다. 만약 Score가 HighScore보다 크다면 HighScore에 Score값을 대입하고싶다.
  (bind _output_get (set `self.Score` (+ Value (`self.Score`))))
  (if (> _output_get (`self.HighScore`))
    (set `self.HighScore` (`self.Score`))))

(fn `LoadHighScore`)

(fn `SaveHighScore`
  ;[1 1 1] 1. SaveGame객체를 만들고 2. 그 객체의 속성에 저장할 값을 대입하고 3. 그것을 슬롯(파일)에 저장.
  (`|ExecutionSequence`
    (:`then_0`
      (bind _returnvalue (`GameplayStatics.CreateSaveGameObject` "/Game/Blueprints/BP_SaveGame.BP_SaveGame_C"))
      (set `self.SaveGameInstance` _returnvalue))
    (:`then_1`
      (set `/Game/Blueprints/BP_SaveGame.SaveHighScore` (`self.HighScore`) (`self.SaveGameInstance`)))
    (:`then_2`
      (`GameplayStatics.SaveGameToSlot` (`self.SaveGameInstance`) (`self.SlotName`)))))

(fn `UserConstructionScript`)